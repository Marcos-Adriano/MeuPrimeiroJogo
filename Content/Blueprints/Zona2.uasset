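; Zona2 is a Simon-style memory puzzle zone where the player repeats a random four-color light-and-beep sequence to open a pair of doors.
; Character overlaps start or reset the game, and each turn plays back one more color via hard-coded delay chains.
; BP_Seringa hits on color colliders are checked per step: mistakes spawn temporary BP_Errou actors and restart with a new sequence.
; Completing four turns triggers applause, flashing lights and timeline-driven doors.
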(event OnComponentBeginOverlap(ColBlue)
  (params (OverlappedComponent :type Primitive%20Component%20Object%20Reference) (OtherActor :type Actor%20Object%20Reference) (OtherComp :type Primitive%20Component%20Object%20Reference) (OtherBodyIndex :type Integer) (bFromSweep :type Boolean) (SweepResult :type Hit%20Result%20Structure%20%28by%20ref%29))
  ;[0.4 0.4 1] Ao acertar o azul seta o valor atual da sequencia como 2
  (Utilities|Casting|CastToBP_Seringa OtherActor)
  (Utilities|Array|SetArrayElem (Variables|Default|GetSequenciaJogador) (Variables|Default|GetAuxVerificaVez) 2 true)
  (CallFunction|AtivarCor (Variables|Default|GetBlueLight))
  (Utilities|FlowControl|Delay 0.5)
  (Math|Integer|IncrementInt (Variables|Default|GetAuxVerificaVez)
    (:%20%20
      (bind _sequenciavalida (CallFunction|VerificaSequencia))
      ;[1 1 1] Se o jogador acertou a sequencia é incrementado 1 em acertos, se errou é penalizado
      (if _sequenciavalida
        (Math|Integer|IncrementInt (Variables|Default|GetAcertos)
          (:%20%20
            ;[1 1 1] Se a quantidade de acertos for igual ao turno quer dizer que o turno acabou e pode jogar o proximo turno, se não for igual só espera o proximo acerto
            (if (== (Variables|Default|GetAcertos) (Variables|Default|GetTurno))
              (Variables|Default|SetAcertos 0)
              (Utilities|Array|Clear (Variables|Default|GetSequenciaJogador))
              (Math|Integer|IncrementInt (Variables|Default|GetTurno)
                (:%20%20
                  (Variables|Default|SetAuxVerificaVez 0)
                  (CallFunction|IniciaTurnoVez :!label _label)
                  (if (== (Variables|Default|GetTurno) 5)
                    (CallFunction|Ganhou)
                    (CallFunction|AbrirPortas)))))))
        (else
          (CallFunction|Errou)
          (Variables|Default|SetAuxVerificaVez 0)
          (CallFunction|SetaSequenciaJogo)
          (Variables|Default|SetTurno 1)
          (Variables|Default|SetAcertos 0)
          (Utilities|Array|Clear (Variables|Default|GetSequenciaJogador))
          (goto _label))))))

(event OnComponentBeginOverlap(ColGreen)
  (params (OverlappedComponent :type Primitive%20Component%20Object%20Reference) (OtherActor :type Actor%20Object%20Reference) (OtherComp :type Primitive%20Component%20Object%20Reference) (OtherBodyIndex :type Integer) (bFromSweep :type Boolean) (SweepResult :type Hit%20Result%20Structure%20%28by%20ref%29))
  ;[0.4 1 0.4] Ao acertar o verde seta o valor atual da sequencia como 1
  (Utilities|Casting|CastToBP_Seringa OtherActor)
  (Utilities|Array|SetArrayElem (Variables|Default|GetSequenciaJogador) (Variables|Default|GetAuxVerificaVez) 1 true)
  (CallFunction|AtivarCor (Variables|Default|GetGreenLight))
  (Utilities|FlowControl|Delay 0.5)
  (Math|Integer|IncrementInt (Variables|Default|GetAuxVerificaVez)
    (:%20%20
      (bind _sequenciavalida (CallFunction|VerificaSequencia))
      ;[1 1 1] Se o jogador acertou a sequencia é incrementado 1 em acertos, se errou é penalizado
      (if _sequenciavalida
        (Math|Integer|IncrementInt (Variables|Default|GetAcertos)
          (:%20%20
            ;[1 1 1] Se a quantidade de acertos for igual ao turno quer dizer que o turno acabou e pode jogar o proximo turno, se não for igual só espera o proximo acerto
            (if (== (Variables|Default|GetAcertos) (Variables|Default|GetTurno))
              (Variables|Default|SetAcertos 0)
              (Utilities|Array|Clear (Variables|Default|GetSequenciaJogador))
              (Math|Integer|IncrementInt (Variables|Default|GetTurno)
                (:%20%20
                  (Variables|Default|SetAuxVerificaVez 0)
                  (CallFunction|IniciaTurnoVez :!label _label)
                  (if (== (Variables|Default|GetTurno) 5)
                    (CallFunction|Ganhou)
                    (CallFunction|AbrirPortas)))))))
        (else
          (CallFunction|Errou)
          (Variables|Default|SetAuxVerificaVez 0)
          (CallFunction|SetaSequenciaJogo)
          (Variables|Default|SetTurno 1)
          (Variables|Default|SetAcertos 0)
          (Utilities|Array|Clear (Variables|Default|GetSequenciaJogador))
          (goto _label))))))

(event OnComponentBeginOverlap(ColYellow)
  (params (OverlappedComponent :type Primitive%20Component%20Object%20Reference) (OtherActor :type Actor%20Object%20Reference) (OtherComp :type Primitive%20Component%20Object%20Reference) (OtherBodyIndex :type Integer) (bFromSweep :type Boolean) (SweepResult :type Hit%20Result%20Structure%20%28by%20ref%29))
  ;[1 1 0.4] Ao acertar o amarelo seta o valor atual da sequencia como 3
  (Utilities|Casting|CastToBP_Seringa OtherActor)
  (Utilities|Array|SetArrayElem (Variables|Default|GetSequenciaJogador) (Variables|Default|GetAuxVerificaVez) 3 true)
  (CallFunction|AtivarCor (Variables|Default|GetYellowLight))
  (Utilities|FlowControl|Delay 0.5)
  (Math|Integer|IncrementInt (Variables|Default|GetAuxVerificaVez)
    (:%20%20
      (bind _sequenciavalida (CallFunction|VerificaSequencia))
      ;[1 1 1] Se o jogador acertou a sequencia é incrementado 1 em acertos, se errou é penalizado
      (if _sequenciavalida
        (Math|Integer|IncrementInt (Variables|Default|GetAcertos)
          (:%20%20
            ;[1 1 1] Se a quantidade de acertos for igual ao turno quer dizer que o turno acabou e pode jogar o proximo turno, se não for igual só espera o proximo acerto
            (if (== (Variables|Default|GetAcertos) (Variables|Default|GetTurno))
              (Variables|Default|SetAcertos 0)
              (Utilities|Array|Clear (Variables|Default|GetSequenciaJogador))
              (Math|Integer|IncrementInt (Variables|Default|GetTurno)
                (:%20%20
                  (Variables|Default|SetAuxVerificaVez 0)
                  (CallFunction|IniciaTurnoVez :!label _label)
                  (if (== (Variables|Default|GetTurno) 5)
                    (CallFunction|Ganhou)
                    (CallFunction|AbrirPortas)))))))
        (else
          (CallFunction|Errou)
          (Variables|Default|SetAuxVerificaVez 0)
          (CallFunction|SetaSequenciaJogo)
          (Variables|Default|SetTurno 1)
          (Variables|Default|SetAcertos 0)
          (Utilities|Array|Clear (Variables|Default|GetSequenciaJogador))
          (goto _label))))))

(event OnComponentBeginOverlap(ColRed)
  (params (OverlappedComponent :type Primitive%20Component%20Object%20Reference) (OtherActor :type Actor%20Object%20Reference) (OtherComp :type Primitive%20Component%20Object%20Reference) (OtherBodyIndex :type Integer) (bFromSweep :type Boolean) (SweepResult :type Hit%20Result%20Structure%20%28by%20ref%29))
  ;[1 0.4187 0.4] Ao acertar o vermelho seta o valor atual da sequencia como 0
  (Utilities|Casting|CastToBP_Seringa OtherActor)
  (Utilities|Array|SetArrayElem (Variables|Default|GetSequenciaJogador) (Variables|Default|GetAuxVerificaVez) 0 true)
  (CallFunction|AtivarCor (Variables|Default|GetRedLight))
  (Utilities|FlowControl|Delay 0.5)
  (Math|Integer|IncrementInt (Variables|Default|GetAuxVerificaVez)
    (:%20%20
      (bind _sequenciavalida (CallFunction|VerificaSequencia))
      ;[1 1 1] Se o jogador acertou a sequencia é incrementado 1 em acertos, se errou é penalizado
      (if _sequenciavalida
        (Math|Integer|IncrementInt (Variables|Default|GetAcertos)
          (:%20%20
            ;[1 1 1] Se a quantidade de acertos for igual ao turno quer dizer que o turno acabou e pode jogar o proximo turno, se não for igual só espera o proximo acerto
            (if (== (Variables|Default|GetAcertos) (Variables|Default|GetTurno))
              (Variables|Default|SetAcertos 0)
              (Utilities|Array|Clear (Variables|Default|GetSequenciaJogador))
              (Math|Integer|IncrementInt (Variables|Default|GetTurno)
                (:%20%20
                  (Variables|Default|SetAuxVerificaVez 0)
                  (CallFunction|IniciaTurnoVez :!label _label)
                  (if (== (Variables|Default|GetTurno) 5)
                    (CallFunction|Ganhou)
                    (CallFunction|AbrirPortas)))))))
        (else
          (CallFunction|Errou)
          (Variables|Default|SetAuxVerificaVez 0)
          (CallFunction|SetaSequenciaJogo)
          (Variables|Default|SetTurno 1)
          (Variables|Default|SetAcertos 0)
          (Utilities|Array|Clear (Variables|Default|GetSequenciaJogador))
          (goto _label))))))

(event OnComponentBeginOverlap(BoxStart)
  (params (OverlappedComponent :type Primitive%20Component%20Object%20Reference) (OtherActor :type Actor%20Object%20Reference) (OtherComp :type Primitive%20Component%20Object%20Reference) (OtherBodyIndex :type Integer) (bFromSweep :type Boolean) (SweepResult :type Hit%20Result%20Structure%20%28by%20ref%29))
  ;[1 1 1] Reset
  (Utilities|Casting|CastToThirdPersonCharacter OtherActor)
  (CallFunction|SetaSequenciaJogo)
  (Variables|Default|SetTurno 1)
  (CallFunction|IniciaTurnoVez))

(event OnComponentBeginOverlap(Box)
  (params (OverlappedComponent :type Primitive%20Component%20Object%20Reference) (OtherActor :type Actor%20Object%20Reference) (OtherComp :type Primitive%20Component%20Object%20Reference) (OtherBodyIndex :type Integer) (bFromSweep :type Boolean) (SweepResult :type Hit%20Result%20Structure%20%28by%20ref%29))
  ;[1 1 1] Sequência criada aleatoriamente com quatro números ao jogador entrar no box do jogo
  (Utilities|Casting|CastToThirdPersonCharacter OtherActor)
  (CallFunction|SetaSequenciaJogo)
  (Utilities|FlowControl|Delay 3.0)
  (Variables|Default|SetTurno 1)
  (CallFunction|IniciaTurnoVez))

(event Custom|IniciaTurnoVez
  (bind _atraso (Variables|Default|GetAtraso))
  (bind _atraso_2 (Variables|Default|GetAtraso))
  (bind _atraso_3 (Variables|Default|GetAtraso))
  (switch int (Variables|Default|GetTurno)
    (:1
      ;[1 1 1] TURNO 1
      (Utilities|FlowControl|Delay (Variables|Default|GetAtraso))
      (bind _cor (CallFunction|NumbertoColor (Utilities|Array|Get(acopy) (Variables|Default|GetSequenciaJogo))))
      (CallFunction|AtivarCor _cor))
    (:2
      ;[1 1 1] TURNO 2
      (Utilities|FlowControl|Delay _atraso_3)
      (bind _cor_2 (CallFunction|NumbertoColor (Utilities|Array|Get(acopy) (Variables|Default|GetSequenciaJogo))))
      (CallFunction|AtivarCor _cor_2)
      (Utilities|FlowControl|Delay _atraso_3)
      (bind _cor_3 (CallFunction|NumbertoColor (Utilities|Array|Get(acopy) (Variables|Default|GetSequenciaJogo) 1)))
      (CallFunction|AtivarCor _cor_3))
    (:3
      ;[1 1 1] TURNO 3
      (Utilities|FlowControl|Delay _atraso_2)
      (bind _cor_4 (CallFunction|NumbertoColor (Utilities|Array|Get(acopy) (Variables|Default|GetSequenciaJogo))))
      (CallFunction|AtivarCor _cor_4)
      (Utilities|FlowControl|Delay _atraso_2)
      (bind _cor_5 (CallFunction|NumbertoColor (Utilities|Array|Get(acopy) (Variables|Default|GetSequenciaJogo) 1)))
      (CallFunction|AtivarCor _cor_5)
      (Utilities|FlowControl|Delay _atraso_2)
      (bind _cor_6 (CallFunction|NumbertoColor (Utilities|Array|Get(acopy) (Variables|Default|GetSequenciaJogo) 2)))
      (CallFunction|AtivarCor _cor_6))
    (:4
      ;[1 1 1] TURNO 4
      (Utilities|FlowControl|Delay _atraso)
      (bind _cor_7 (CallFunction|NumbertoColor (Utilities|Array|Get(acopy) (Variables|Default|GetSequenciaJogo))))
      (CallFunction|AtivarCor _cor_7)
      (Utilities|FlowControl|Delay _atraso)
      (bind _cor_8 (CallFunction|NumbertoColor (Utilities|Array|Get(acopy) (Variables|Default|GetSequenciaJogo) 1)))
      (CallFunction|AtivarCor _cor_8)
      (Utilities|FlowControl|Delay _atraso)
      (bind _cor_9 (CallFunction|NumbertoColor (Utilities|Array|Get(acopy) (Variables|Default|GetSequenciaJogo) 2)))
      (CallFunction|AtivarCor _cor_9)
      (Utilities|FlowControl|Delay _atraso)
      (bind _cor_10 (CallFunction|NumbertoColor (Utilities|Array|Get(acopy) (Variables|Default|GetSequenciaJogo) 3)))
      (CallFunction|AtivarCor _cor_10))))

(event Custom|SetaSequenciaJogo
  ;[1 1 1] Função que define a sequência de 4 números (cores) do jogo
  (for _index (range 0 3)
    (bind _output_get (Variables|Default|SetEscolhaRand (Math|Random|RandomIntegerinRange 0 3)))
    (Utilities|Array|SetArrayElem (Variables|Default|GetSequenciaJogo) _index _output_get)))

(event Custom|Ganhou
  ;[1 1 1] Piscar Luz e som correspondente
  (CallFunction|Aplauses)
  (CallFunction|Parabens))

(event Custom|AtivarCor
  (params (LuzCor :type Spot%20Light%20Component%20Object%20Reference%20%28by%20ref%29))
  ;[1 1 1] Piscar Luz e som correspondente
  (Rendering|SetVisibility LuzCor true false)
  (if (== LuzCor (Variables|Default|GetRedLight))
    (Audio|PlaySound2D "/Game/Sons/Genius/Beep0_Cue.Beep0_Cue" 1.0 1.0 0.0 0 0)
    (Utilities|FlowControl|Delay 0.4 :!label _label)
    (Rendering|SetVisibility LuzCor false false)
    (Utilities|FlowControl|Delay 0.6)
    (elif (== LuzCor (Variables|Default|GetGreenLight))
      (Audio|PlaySound2D "/Game/Sons/Genius/Beep1_Cue.Beep1_Cue" 1.0 1.0 0.0 0 0)
      (goto _label)
      (elif (== LuzCor (Variables|Default|GetBlueLight))
        (Audio|PlaySound2D "/Game/Sons/Genius/Beep2_Cue.Beep2_Cue" 1.0 1.0 0.0 0 0)
        (goto _label)
        (elif (== LuzCor (Variables|Default|GetYellowLight))
          (Audio|PlaySound2D "/Game/Sons/Genius/Beep3_Cue.Beep3_Cue" 1.0 1.0 0.0 0 0)
          (goto _label))))))

(event Custom|Aplauses
  ;[1 1 1] Piscar Luz e som correspondente
  (Audio|PlaySound2D "/Game/Sons/Genius/aplauses_Cue.aplauses_Cue" 1.0 1.0 0.0 0 0))

(event Custom|Parabens
  ;[1 1 1] Piscar Luz e som correspondente
  (Rendering|SetVisibility (Variables|Default|GetGreenLight) true false)
  (Utilities|FlowControl|Delay 0.3)
  (Rendering|SetVisibility (Variables|Default|GetYellowLight) false false)
  (Utilities|FlowControl|Delay 0.3)
  (Rendering|SetVisibility (Variables|Default|GetGreenLight) true false)
  (Utilities|FlowControl|Delay 0.3)
  (Rendering|SetVisibility (Variables|Default|GetYellowLight) false false)
  (Utilities|FlowControl|Delay 0.3)
  (Rendering|SetVisibility (Variables|Default|GetGreenLight) true false)
  (Utilities|FlowControl|Delay 0.3)
  (Rendering|SetVisibility (Variables|Default|GetYellowLight) false false)
  (Utilities|FlowControl|Delay 0.3)
  (Rendering|SetVisibility (Variables|Default|GetGreenLight) true false)
  (Utilities|FlowControl|Delay 0.3)
  (Rendering|SetVisibility (Variables|Default|GetYellowLight) false false)
  (Utilities|FlowControl|Delay 0.3)
  (Rendering|SetVisibility (Variables|Default|GetGreenLight) true false)
  (Utilities|FlowControl|Delay 0.3)
  (Rendering|SetVisibility (Variables|Default|GetYellowLight) false false)
  (Utilities|FlowControl|Delay 0.3)
  (Rendering|SetVisibility (Variables|Default|GetGreenLight) true false)
  (Utilities|FlowControl|Delay 0.3)
  (Rendering|SetVisibility (Variables|Default|GetYellowLight) false false))

(event Custom|Errou
  (Audio|PlaySound2D "/Game/Sons/Genius/wrong-answer_Cue.wrong-answer_Cue" 1.0 1.0 0.0 0 0)
  (Utilities|FlowControl|Sequence
    (:then_0
      (bind _returnvalue (Game|SpawnActorfromClass "/Game/Blueprints/BP_Errou.BP_Errou_C" (Transformation|GetWorldTransform (Variables|Default|GetArrow2)) "Undefined" 0 0))
      (Utilities|FlowControl|Delay 2.0)
      (Actor|DestroyActor _returnvalue))
    (:then_1
      (bind _returnvalue_2 (Game|SpawnActorfromClass "/Game/Blueprints/BP_Errou.BP_Errou_C" (Transformation|GetWorldTransform (Variables|Default|GetArrow3)) "Undefined" 0 0))
      (Utilities|FlowControl|Delay 2.0)
      (Actor|DestroyActor _returnvalue_2))))

(event Custom|AbrirPortas
  (bind _portaesq (Variables|Default|GetPortaEsq))
  (bind _portadir (Variables|Default|GetPortaDir))
  (bind _returnvalue (Transformation|GetWorldLocation _portadir))
  (bind _returnvalue_2 (Transformation|GetWorldLocation _portaesq))
  ;[1 1 1] Comment
  (bind _localdir (Timeline|Timeline_0 Play)
    (:Update
      (Transformation|SetWorldLocation _portadir (Math|Vector|MakeVector (.x _returnvalue) _localdir (.z _returnvalue)) false false)
      (bind _locesq (Timeline|Timeline_1 Play)
        (:Update
          (Transformation|SetWorldLocation _portaesq (Math|Vector|MakeVector (.x _returnvalue_2) _locesq (.z _returnvalue_2)) false false))))))

(fn ConstructionScript)

(fn NumbertoColor
  (params (Numero :type Integer))
  (if (== Numero 0)
    (return (Variables|Default|GetRedLight))
    (elif (== Numero 1)
      (return (Variables|Default|GetGreenLight))
      (elif (== Numero 2)
        (return (Variables|Default|GetBlueLight))
        (elif (== Numero 3)
          (return (Variables|Default|GetYellowLight))
          (else
            (return 0)))))))

(fn VerificaSequencia
  (bind _auxverificavez (Variables|Default|GetAuxVerificaVez))
  (bind _returnvalue (- _auxverificavez 1))
  (if (== (Utilities|Array|Get(acopy) (Variables|Default|GetSequenciaJogo) _returnvalue) (Utilities|Array|Get(acopy) (Variables|Default|GetSequenciaJogador) _returnvalue))
    (return true)
    (else
      (return false))))

(fn TurnoVez)