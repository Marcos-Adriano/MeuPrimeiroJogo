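; Final double door that opens once the ThirdPersonGameMode's InimigosRestantes count reaches zero and ends the game when the player walks into its trigger box.
; Tick polls that count and fires AbrirPortas once, which destroys a plane, brightens a point light and rotates both door leaves through two timelines.
; Overlap by the ThirdPersonCharacter swaps all widgets for the TelaFimJogo end screen, then pauses after a brief delay and shows the cursor.
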(event OnComponentBeginOverlap(Box)
  (params (OverlappedComponent :type Primitive%20Component%20Object%20Reference) (OtherActor :type Actor%20Object%20Reference) (OtherComp :type Primitive%20Component%20Object%20Reference) (OtherBodyIndex :type Integer) (bFromSweep :type Boolean) (SweepResult :type Hit%20Result%20Structure%20%28by%20ref%29))
  (Utilities|Casting|CastToThirdPersonCharacter OtherActor)
  (bind _returnvalue (UserInterface|CreateWidget "/Game/Widgets/TelaFimJogo.TelaFimJogo_C"))
  (Viewport|RemoveAllWidgets)
  (UserInterface|Viewport|AddtoViewport _returnvalue 0)
  (Utilities|FlowControl|Delay 0.2)
  (Game|SetGamePaused true)
  (Variables|/Script/Engine.PlayerController|SetbShowMouseCursor (Game|GetPlayerController 0) true))

(event Custom|AbrirPortas
  (bind _portadir (Variables|Default|GetPortaDir))
  (bind _portaesq (Variables|Default|GetPortaEsq))
  (bind _relativerotation (Variables|/Script/Engine.SceneComponent|GetRelativeRotation _portaesq))
  (bind _relativerotation_2 (Variables|/Script/Engine.SceneComponent|GetRelativeRotation _portadir))
  (Utilities|FlowControl|Sequence
    (:then_0
      (Components|DestroyComponent (Variables|Default|GetPlane))
      (Rendering|Components|Light|SetIntensity (Variables|Default|GetPointLight) 1e+05))
    (:then_1
      (bind _rotacaodir (Timeline|AbrirDir PlayFromStart)
        (:Update
          (Transformation|SetRelativeRotation _portadir (Math|Rotator|MakeRotator (.roll _relativerotation_2) (.pitch _relativerotation_2) _rotacaodir) false false))))
    (:then_2
      (bind _rotacaoesq (Timeline|AbrirEsq PlayFromStart)
        (:Update
          (Transformation|SetRelativeRotation _portaesq (Math|Rotator|MakeRotator (.roll _relativerotation) (.pitch _relativerotation) _rotacaoesq) false false))))))

(event EventTick
  (params (DeltaSeconds :type Float%20%28single-precision%29))
  (bind _asthird_person_game_mode (Utilities|Casting|CastToThirdPersonGameMode (Game|GetGameMode)))
  (if (<= (Variables|/Game/ThirdPersonBP/Blueprints/ThirdPersonGameMode.ThirdPersonGameMode_C|GetInimigosRestantes _asthird_person_game_mode) 0)
    (Utilities|FlowControl|DoOnce false
      (:Completed
        (CallFunction|AbrirPortas)))))

(fn ConstructionScript)