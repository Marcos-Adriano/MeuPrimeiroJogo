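; BP_Seringa is a short-lived syringe actor, apparently a projectile, that damages enemies it hits.
; On a hit, it applies fixed damage if the other actor's class is exactly the boss, ranged or melee enemy Blueprint.
; Any hit spawns a scaled-down explosion particle effect and destroys the actor, while a lifespan set at BeginPlay removes it if nothing is hit.
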(event EventBeginPlay
  (Actor|SetLifeSpan 1e+01))

(event Collision|EventHit
  (params (MyComp :type Primitive%20Component%20Object%20Reference) (Other :type Actor%20Object%20Reference) (OtherComp :type Primitive%20Component%20Object%20Reference) (bSelfMoved :type Boolean) (HitLocation :type Vector :default "0, 0, 0") (HitNormal :type Vector :default "0, 0, 0") (NormalImpulse :type Vector :default "0, 0, 0") (Hit :type Hit%20Result%20Structure%20%28by%20ref%29))
  (bind _returnvalue (Utilities|GetClass Other))
  (if (Math|Boolean|ORBoolean (== _returnvalue "/Game/Personagens/Boss/BP_BOSS.BP_BOSS_C") (== _returnvalue "/Game/Personagens/Ranged/BP_RANGED.BP_RANGED_C") (== _returnvalue "/Game/MELEE_IA/BP_MELEE.BP_MELEE_C"))
    (Game|Damage|ApplyDamage Other 15.0 0 self "/Script/Engine.DamageType"))
  (Effects|SpawnEmitteratLocation "/Game/StarterContent/Particles/P_Explosion.P_Explosion" (Transformation|GetActorLocation) "0, 0, 0" "0.500000,0.500000,0.500000")
  (Actor|DestroyActor))

(fn ConstructionScript)