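; BP_PassagemZona3 is a passage with a pair of sliding doors that open when the player's ThirdPersonCharacter enters a trigger area and close when it leaves.
; Overlapping AreaPortas plays one timeline per door, and ending the overlap reverses both.
; Each timeline update sets only its door's world X position from an absolute track value, keeping Y and Z, so the motion is tied to where the doors sit in the level.
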(event OnComponentBeginOverlap(AreaPortas)
  (params (OverlappedComponent :type Primitive%20Component%20Object%20Reference) (OtherActor :type Actor%20Object%20Reference) (OtherComp :type Primitive%20Component%20Object%20Reference) (OtherBodyIndex :type Integer) (bFromSweep :type Boolean) (SweepResult :type Hit%20Result%20Structure%20%28by%20ref%29))
  (bind _portadir (Variables|Default|GetPortaDir))
  (bind _portaesq (Variables|Default|GetPortaEsq))
  (bind _returnvalue (Transformation|GetWorldLocation _portaesq))
  (bind _returnvalue_2 (Transformation|GetWorldLocation _portadir))
  (Utilities|Casting|CastToThirdPersonCharacter OtherActor)
  (Utilities|FlowControl|Sequence
    (:then_0
      (bind _locxesq (Timeline|PortaEsquerda Play)
        (:Update
          (Transformation|SetWorldLocation _portaesq (Math|Vector|MakeVector _locxesq (.y _returnvalue) (.z _returnvalue)) false false))))
    (:then_1
      (bind _locxdir (Timeline|PortaDireita Play)
        (:Update
          (Transformation|SetWorldLocation _portadir (Math|Vector|MakeVector _locxdir (.y _returnvalue_2) (.z _returnvalue_2)) false false))))))

(event OnComponentEndOverlap(AreaPortas)
  (params (OverlappedComponent :type Primitive%20Component%20Object%20Reference) (OtherActor :type Actor%20Object%20Reference) (OtherComp :type Primitive%20Component%20Object%20Reference) (OtherBodyIndex :type Integer))
  (bind _portadir (Variables|Default|GetPortaDir))
  (bind _portaesq (Variables|Default|GetPortaEsq))
  (bind _returnvalue (Transformation|GetWorldLocation _portaesq))
  (bind _returnvalue_2 (Transformation|GetWorldLocation _portadir))
  (Utilities|Casting|CastToThirdPersonCharacter OtherActor)
  (Utilities|FlowControl|Sequence
    (:then_0
      (bind _locxdir (Timeline|PortaDireita Reverse)
        (:Update
          (Transformation|SetWorldLocation _portadir (Math|Vector|MakeVector _locxdir (.y _returnvalue_2) (.z _returnvalue_2)) false false))))
    (:then_1
      (bind _locxesq (Timeline|PortaEsquerda Reverse)
        (:Update
          (Transformation|SetWorldLocation _portaesq (Math|Vector|MakeVector _locxesq (.y _returnvalue) (.z _returnvalue)) false false))))))

(fn ConstructionScript)