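; BP_Errou is a hazard actor that applies environmental damage to the third-person character when it overlaps the actor.
; A looping timer started on BeginPlay makes a fire light flicker just above it.
; Each pulse spawns a separate point light actor and destroys it after a short delay, rather than toggling a component.
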(event Custom|LuzFogo
  (bind _returnvalue (Game|SpawnActorfromClass "/Game/Blueprints/MyPointLight_Fire.MyPointLight_Fire_C" (Math|Transform|MakeTransform (+ (Transformation|GetActorLocation) "0, 0,40.000000") "0, 0, 0" "1,1,1") "Undefined" 0 0))
  (Utilities|FlowControl|Delay 0.4)
  (Actor|DestroyActor _returnvalue))

(event Collision|EventActorBeginOverlap
  (params (OtherActor :type Actor%20Object%20Reference))
  ;[1 1 1] Aplica dano ao jogador passar por cima
  (bind _asthird_person_character (Utilities|Casting|CastToThirdPersonCharacter OtherActor))
  (Game|Damage|ApplyDamage _asthird_person_character 4e+01 0 self "/Engine/EngineDamageTypes/DmgTypeBP_Environmental.DmgTypeBP_Environmental_C"))

(event EventBeginPlay
  (Utilities|Time|SetTimerbyEvent (delegate Custom|LuzFogo) 0.8 true))

(fn ConstructionScript)