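; BP_RANGED is a ranged enemy character that fires at a given target and can be killed.
; ShootEnemy traces toward the target, plays a muzzle flash and spawns a Municao_RANGED projectile from the gun socket, aimed at the impact point or target.
; Tick updates the widget health bar.
; Damage plays a hit sound; death decrements the game mode's remaining-enemy count, ragdolls the mesh and destroys the actor after a delay.
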(event Custom|Shoot%20Enemy
  (params (EnemyToShoot :type Actor%20Object%20Reference))
  (bind _gunmesh (Variables|Default|GetGunMesh))
  (bind _returnvalue (Transformation|GetSocketLocation _gunmesh "Cano"))
  (Utilities|FlowControl|Sequence
    (:then_0
      (Variables|Default|SetEnd (Transformation|GetActorLocation EnemyToShoot))
      (Variables|Default|SetStart (Transformation|GetActorLocation)))
    (:then_1
      (bind (_outhit _returnvalue_2) (Collision|LineTraceByChannel (Variables|Default|GetStart) (Variables|Default|GetEnd) "TraceTypeQuery2" false 0 "None"))
      (if _returnvalue_2
        (Variables|Default|SetEnd (.ImpactPoint (Collision|BreakHitResult _outhit)))))
    (:then_2
      (CallFunction|PlayShootFX))
    (:then_3
      (Game|SpawnActorfromClass "/Game/Personagens/Ranged/Weapon/Municao_RANGED.Municao_RANGED_C" (Math|Transform|MakeTransform _returnvalue (Math|Rotator|FindLookatRotation _returnvalue (Variables|Default|GetEnd)) "1,1,1") "AlwaysSpawn" 0 0))))

(event Custom|Play%20Shoot%20FX
  (bind _gunmesh (Variables|Default|GetGunMesh))
  (Effects|SpawnEmitteratLocation "/Game/InfinityBladeEffects/Effects/FX_Mobile/Fire/combat/MuzzleFlash.MuzzleFlash" (Transformation|GetSocketLocation _gunmesh "Cano") (Transformation|GetSocketRotation _gunmesh "Cano")))

(event Game|Damage|EventAnyDamage
  (params (Damage :type Float%20%28single-precision%29) (DamageType :type Damage%20Type%20Object%20Reference) (InstigatedBy :type Controller%20Object%20Reference) (DamageCauser :type Actor%20Object%20Reference))
  (bind _mesh (Variables|Character|GetMesh))
  (Utilities|FlowControl|Sequence
    (:then_0
      (if (not (Variables|Default|GetEstaMorto))
        (Audio|PlaySoundatLocation "/Game/Sons/Sons/zombie-hit_Cue.zombie-hit_Cue" (Transformation|GetActorLocation) "0, 0, 0" 1.0 1.0 0.0 0 0 0)))
    (:then_1
      (Variables|Default|SetHealth (- (Variables|Default|GetHealth) Damage))
      (if (< (Variables|Default|GetHealth) 0.0)
        (Variables|Default|SetEstaMorto true)
        (bind _asthird_person_game_mode (Utilities|Casting|CastToThirdPersonGameMode (Game|GetGameMode)))
        (Math|Integer|DecrementInt (Variables|/Game/ThirdPersonBP/Blueprints/ThirdPersonGameMode.ThirdPersonGameMode_C|GetInimigosRestantes _asthird_person_game_mode)
          (:%20%20
            (Physics|SetSimulatePhysics (Variables|Character|GetMesh) true)
            (Collision|SetCollisionProfileName _mesh "Ragdoll" true :!class /Script/Engine.PrimitiveComponent)
            (Collision|SetCollisionResponsetoChannel _mesh "ECC_Pawn" "ECR_Block")
            (Rendering|SetVisibility (Variables|Default|GetWidget) false false)
            (Components|DestroyComponent (Variables|Collision|GetCapsuleComponent))
            (Utilities|FlowControl|Delay 1e+01)
            (Actor|DestroyActor)))))))

(event EventTick
  (params (DeltaSeconds :type Float%20%28single-precision%29))
  (bind _ashud_enemy (Utilities|Casting|CastToHUD_Enemy (UserInterface|GetUserWidgetObject (Variables|Default|GetWidget))))
  (Progress|SetPercent (Variables|/Game/Widgets/HUD_Enemy.HUD_Enemy_C|GetEnemyProgressBar _ashud_enemy) (/ (Variables|Default|GetHealth) 9e+01)))

(event EventBeginPlay
  (Transformation|AttachComponentToComponent (Variables|Default|GetGunMesh) (Variables|Character|GetMesh) "WeaponSocket" "SnapToTarget" "SnapToTarget" "SnapToTarget" true))

(fn ConstructionScript)