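; Boss enemy character that chases the player on sight, performs a timed double melee attack and dies into a ragdoll.
; Pawn sensing sets the target and raises run speed, while Attack opens a brief damage window for the box overlap and then lowers speed.
; Incoming damage plays a hit sound and drains health, shown on a widget bar.
; Death decrements the game mode's remaining-enemy count and destroys the actor after a delay.
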(event OnSeePawn(PawnSensing)
  (params (Pawn :type Pawn%20Object%20Reference))
  (bind _asthird_person_character (Utilities|Casting|CastToThirdPersonCharacter Pawn))
  (Variables|Default|SetTargetPlayer _asthird_person_character)
  (Variables|/Script/Engine.CharacterMovementComponent|SetMaxWalkSpeed (Variables|/Script/Engine.Character|GetCharacterMovement self) 7.5e+02))

(event OnComponentBeginOverlap(Box)
  (params (OverlappedComponent :type Primitive%20Component%20Object%20Reference) (OtherActor :type Actor%20Object%20Reference) (OtherComp :type Primitive%20Component%20Object%20Reference) (OtherBodyIndex :type Integer) (bFromSweep :type Boolean) (SweepResult :type Hit%20Result%20Structure%20%28by%20ref%29))
  (bind _asthird_person_character (Utilities|Casting|CastToThirdPersonCharacter OtherActor))
  (if (Variables|Default|GetIsAttacking)
    (Game|Damage|ApplyDamage _asthird_person_character 3e+01 0 self)))

(event Custom|Attack
  (if (> (Variables|/Game/Blueprints/ThirdPersonCharacter.ThirdPersonCharacter_C|GetHealth (Variables|Default|GetTargetPlayer)) 0.0)
    (Components|Animation|PlayAnimation (Variables|Character|GetMesh) "/Game/Personagens/Boss/Animacoes/BOSS_AttackDouble.BOSS_AttackDouble" false)
    (Utilities|FlowControl|Delay 1.1)
    (Variables|Default|SetIsAttacking true)
    (Utilities|FlowControl|Delay 1.1)
    (Variables|Default|SetIsAttacking false)
    (Components|Animation|SetAnimationMode (Variables|Character|GetMesh) "AnimationBlueprint"))
  (Variables|/Script/Engine.CharacterMovementComponent|SetMaxWalkSpeed (Variables|/Script/Engine.Character|GetCharacterMovement self) 325.0))

(event Game|Damage|EventAnyDamage
  (params (Damage :type Float%20%28single-precision%29) (DamageType :type Damage%20Type%20Object%20Reference) (InstigatedBy :type Controller%20Object%20Reference) (DamageCauser :type Actor%20Object%20Reference))
  (bind _mesh (Variables|Character|GetMesh))
  (Utilities|FlowControl|Sequence
    (:then_0
      (if (not (Variables|Default|GetEstaMorto))
        (Audio|PlaySoundatLocation "/Game/Sons/Sons/zombie-hit_Cue.zombie-hit_Cue" (Transformation|GetActorLocation) "0, 0, 0" 1.0 1.0 0.0 0 0 0)))
    (:then_1
      (bind _output_get (Variables|Default|SetHealth (- (Variables|Default|GetHealth) Damage)))
      (if (< _output_get 0.0)
        (Variables|Default|SetEstaMorto true)
        (bind _asthird_person_game_mode (Utilities|Casting|CastToThirdPersonGameMode (Game|GetGameMode)))
        (Math|Integer|DecrementInt (Variables|/Game/ThirdPersonBP/Blueprints/ThirdPersonGameMode.ThirdPersonGameMode_C|GetInimigosRestantes _asthird_person_game_mode)
          (:%20%20
            (Physics|SetSimulatePhysics (Variables|Character|GetMesh) true)
            (Collision|SetCollisionProfileName _mesh "Ragdoll" true :!class /Script/Engine.PrimitiveComponent)
            (Collision|SetCollisionResponsetoChannel _mesh "ECC_Pawn" "ECR_Block")
            (Rendering|SetVisibility (Variables|Default|GetWidget) false false)
            (Components|DestroyComponent (Variables|Collision|GetCapsuleComponent))
            (Utilities|FlowControl|Delay 15.0)
            (Actor|DestroyActor)))))))

(event EventTick
  (params (DeltaSeconds :type Float%20%28single-precision%29))
  (bind _ashud_enemy (Utilities|Casting|CastToHUD_Enemy (UserInterface|GetUserWidgetObject (Variables|Default|GetWidget))))
  (Progress|SetPercent (Variables|/Game/Widgets/HUD_Enemy.HUD_Enemy_C|GetEnemyProgressBar _ashud_enemy) (/ (Variables|Default|GetHealth) 3e+02)))

(fn ConstructionScript)